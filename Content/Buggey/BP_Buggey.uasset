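; BP_Buggey is the player's racing buggy, with throttle, steering, two hammer-swing animations and a Q key that multiplies velocity tenfold.
; Before the race, Tick pins it still while throttle charges a boost shown by wheel sparks and smoke.
; At race start, a charge below the overcharge limit gives a one-time proportional launch.
; If flipped and stuck, it destroys itself so the player controller respawns it.
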(event `Key|Q`
  (params (Key :type "Key Structure" :default "AnyKey"))
  (bind _mesh (`self.Mesh`))
  (:`Pressed`
    (bind _returnvalue (`PrimitiveComponent.GetPhysicsLinearVelocity` _mesh "None"))
    (`PrimitiveComponent.SetPhysicsLinearVelocity` _mesh (* _returnvalue 10.0) false "None")))

(event `self.ReceiveTick`
  (params (DeltaSeconds :type "Float (single-precision)"))
  (`self.Boosting`)
  ;[1 1 1] Disable input when the race is finished
  (if (`/Game/Blueprints/MyPlayerController.RaceComplete` (`self.ControllerReference`))
    (`WheeledVehicleMovementComponent.SetThrottleInput` (`self.VehicleMovement`) 0.0)
    (else
      ;[1 1 1] Checking if player has flipped car and will call respawn player
      (bind _playerisstuck (`self.RespawnCheck`))
      (if _playerisstuck
        (`KismetSystemLibrary.Delay` 3.0)
        (bind _playerisstuck_2 (`self.RespawnCheck`))
        (if _playerisstuck_2
          (`self.K2_DestroyActor`))))))

(event `self.ReceiveDestroyed`
  ;[1 1 1] Checking if player has flipped car and will call respawn player
  (`/Game/Blueprints/MyPlayerController.RespawnVehicle` (`self.ControllerReference`)))

(event `self.ReceiveBeginPlay`
  ;[1 1 1] Disable Input on racestart
  (bind _asmy_player_controller (cast `/Game/Blueprints/MyPlayerController` (`GameplayStatics.GetPlayerController` 0)))
  (bind _output_get (set `self.ControllerReference` _asmy_player_controller))
  (set `/Game/Blueprints/MyPlayerController.ReSpawnLocation` (`self.GetTransform`) _output_get))

(event `InputAction|AntiSwing`
  (params (Key :type "Key Structure" :default "AnyKey"))
  ;[1 1 1] Hammer
  (:`Pressed`
    (if (not (`SkeletalMeshComponent.IsPlaying` (`self.Hammer`)))
      (`SkeletalMeshComponent.PlayAnimation` (`self.Hammer`) "/Game/Buggey/AntiHammerSwing_Anim.AntiHammerSwing_Anim" false))))

(event `InputAxis|Forward`
  (params (AxisValue :type "Float (single-precision)"))
  (bind _acceleration (`self.Acceleration`))
  ;[1 1 1] Movement
  (bind _output_get (set `self.Acceleration` AxisValue))
  (`WheeledVehicleMovementComponent.SetThrottleInput` (`self.VehicleMovement`) _output_get)
  ;[1 1 1] Charge boost before race
  (if (`/Game/Blueprints/MyPlayerController.RaceStart` (`self.ControllerReference`))
    _
    (elif (> _acceleration 0.0)
      (set `self.BoostStart` (+ (`self.BoostStart`) _acceleration))
      (else
        (set `self.BoostStart` 0.0)))))

(event `InputAction|Swing`
  (params (Key :type "Key Structure" :default "AnyKey"))
  ;[1 1 1] Hammer
  (:`Pressed`
    (if (not (`SkeletalMeshComponent.IsPlaying` (`self.Hammer`)))
      (`SkeletalMeshComponent.PlayAnimation` (`self.Hammer`) "/Game/Buggey/HammerSwing_Anim.HammerSwing_Anim" false))))

(event `InputAxis|Right`
  (params (AxisValue :type "Float (single-precision)"))
  ;[1 1 1] Movement
  (`WheeledVehicleMovementComponent.SetSteeringInput` (`self.VehicleMovement`) AxisValue))

(fn `Boosting`
  (bind _booststart (`self.BoostStart`))
  (bind _booststart_2 (`self.BoostStart`))
  (bind _returnvalue (- (`self.BoostStart`) 140.0))
  (if (< (`self.BoostStart`) 140.0)
    (`ParticleSystemComponent.SetVectorParameter` (`self.LeftWheelBoostSparks`) "SparkColour" (`KismetMathLibrary.MakeVector` 1.0 (- 1.0 (/ (`self.BoostStart`) 140.0))))
    (`ParticleSystemComponent.SetVectorParameter` (`self.RightWheelBoostSparks`) "SparkColour" (`KismetMathLibrary.MakeVector` 1.0 (- 1.0 (/ (`self.BoostStart`) 140.0))))
    (else
      (`ParticleSystemComponent.SetVectorParameter` (`self.LeftWheelBoostSparks`) "SparkColour" (`KismetMathLibrary.MakeVector` (- 1.0 (/ _returnvalue 20.0)) 0.0 (/ _returnvalue 40.0)))
      (`ParticleSystemComponent.SetVectorParameter` (`self.RightWheelBoostSparks`) "SparkColour" (`KismetMathLibrary.MakeVector` (- 1.0 (/ _returnvalue 20.0)) 0.0 (/ _returnvalue 40.0)))))
  (`ParticleSystemComponent.SetFloatParameter` (`self.LeftWheelBoostSparks`) "Boosting" (* (`self.BoostStart`) 1.5))
  (`ParticleSystemComponent.SetFloatParameter` (`self.RightWheelBoostSparks`) "Boosting" (* (`self.BoostStart`) 1.5))
  (if (`/Game/Blueprints/MyPlayerController.RaceStart` (`self.ControllerReference`))
    (if (and (> 160.0 _booststart_2) (> _booststart_2 0.0) (not (`self.HasBoosted`)))
      (`PrimitiveComponent.SetAllPhysicsLinearVelocity` (`self.Mesh`) (* (`self.BoostSpeed`) (/ _booststart 160.0)) false)
      (else
        (set `self.BoostStart` (- _booststart 0.5))))
    (set `self.HasBoosted` true)
    (`ParticleSystemComponent.SetFloatParameter` (`self.RightWheelSmoke`) "SmokeAlpha" 0.0)
    (`ParticleSystemComponent.SetFloatParameter` (`self.LeftWheelSmoke`) "SmokeAlpha" 0.0)
    (else
      (`PrimitiveComponent.SetAllPhysicsLinearVelocity` (`self.Mesh`) (0.0 0.0 0.0) false)
      (`ParticleSystemComponent.SetFloatParameter` (`self.LeftWheelSmoke`) "SmokeAlpha" (/ (`WheeledVehicleMovementComponent.GetEngineRotationSpeed` (`self.VehicleMovement`)) 1000.0))
      (`ParticleSystemComponent.SetFloatParameter` (`self.RightWheelSmoke`) "SmokeAlpha" (/ (`WheeledVehicleMovementComponent.GetEngineRotationSpeed` (`self.VehicleMovement`)) 1000.0)))))

(fn `RespawnCheck`
  (returns (PlayerIsStuck :type Boolean))
  ;[1 1 1] Check and see if the player is stuck upside down
  (if (and (< (`KismetMathLibrary.Dot_VectorVector` (`self.GetActorUpVector`) (0.0 0.0 1.0)) 0.5) (< (`WheeledVehicleMovementComponent.GetForwardSpeed` (`self.VehicleMovement`)) 0.5))
    (set `self.Stuck?` true)
    (else
      (set `self.Stuck?` false)))
  (return (`self.Stuck?`)))

(fn `TurningEffects`)

(fn `UserConstructionScript`)