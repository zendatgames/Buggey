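; Checkpoint is a race checkpoint actor that detects when a BP_Buggey drives through it in the correct direction.
; On overlap, it compares the buggy's velocity against the Arrow component's forward vector with a dot product, so only forward passes count.
; A valid pass fires the CheckpointCleared dispatcher with its CheckpointNumber, then turns off the trigger's overlap events so it counts once.
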(event `self.Trigger.OnComponentBeginOverlap`
  (params (OverlappedComponent :type "PrimitiveComponent Object Reference") (OtherActor :type "Actor Object Reference") (OtherComp :type "PrimitiveComponent Object Reference") (OtherBodyIndex :type Integer) (bFromSweep :type Boolean) (SweepResult :type "HitResult Structure (by ref)"))
  ;[1 1 1] Checkpoints
  (bind _asbp_buggey (cast `/Game/Buggey/BP_Buggey` OtherActor))
  (if (> (`KismetMathLibrary.Dot_VectorVector` (`self.GetVelocity` _asbp_buggey) (`KismetMathLibrary.Conv_RotatorToVector` (`SceneComponent.K2_GetComponentRotation` (`self.Arrow`)))) 0.0)
    (`self.CheckpointCleared` (`self.CheckpointNumber`))
    (set `PrimitiveComponent.bGenerateOverlapEvents` false (`self.Trigger`))))

(fn `UserConstructionScript`)