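; Out-of-bounds actor that destroys any actor overlapping it and tallies the money lost over the table.
; Each overlapped actor's tags are converted to integers and added to both MoneyLost and the MyPlayerController's Score, with the controller's MoneyLostTxt updated to match.
; Tick calls LowerWall on CardWall every frame while MoneyLost is zero or above, rather than once on reaching the target.
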(event `self.ReceiveBeginPlay`
  (bind _asmy_player_controller (cast `/Game/Blueprints/MyPlayerController` (`GameplayStatics.GetPlayerController` 0)))
  (set `self.PlayerControllerRef` _asmy_player_controller))

(event `self.ReceiveActorBeginOverlap`
  (params (OtherActor :type "Actor Object Reference"))
  (bind _playercontrollerref (`self.PlayerControllerRef`))
  ;[1 1 1] Keeps track of money lost over the table, passes that value to PlayerController and destroys actors that fall
  (bind _output_get (set `self.OverlappedActor` OtherActor))
  (for _array_element (`Actor.Tags` _output_get)
    (bind _returnvalue (`KismetStringLibrary.Conv_StringToInt` (`KismetStringLibrary.Conv_NameToString` _array_element)))
    (bind _output_get_2 (set `self.MoneyLost` (+ (`self.MoneyLost`) _returnvalue)))
    (set `/Game/Blueprints/MyPlayerController.MoneyLostTxt` (`KismetTextLibrary.Conv_IntToText` _output_get_2) _playercontrollerref)
    (set `/Game/Blueprints/MyPlayerController.Score` (+ _returnvalue (`/Game/Blueprints/MyPlayerController.Score` _playercontrollerref)) _playercontrollerref))
  (`self.K2_DestroyActor` (`self.OverlappedActor`)))

(event `self.ReceiveTick`
  (params (DeltaSeconds :type "Float (single-precision)"))
  ;[1 1 1] Calls LowerWall custom event to lower CardWall when target is reached
  (if (>= (`self.MoneyLost`) 0)
    (`/Game/Racetrack/CardWall.LowerWall` (`self.CardWall`))))

(fn `UserConstructionScript`
  (`parent.UserConstructionScript`))