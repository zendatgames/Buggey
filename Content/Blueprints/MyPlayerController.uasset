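; Player controller for a buggy lap race that runs the countdown, race and lap timers, HUD and race restart.
; Timelines drive the clocks and their display text, while lap updates record each of three lap times and check lap and race records.
; Best times persist through a SaveGame slot and can be reset to defaults before the race starts.
; It also tracks vehicle speed and respawns and possesses a new buggy.
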(event `self.ReceiveTick`
  (params (DeltaSeconds :type "Float (single-precision)"))
  ;[1 1 1] Set the Buggey's Speed Variable
  (set `self.BuggeySpeed` (`WheeledVehicleMovementComponent.GetForwardSpeed` (`WheeledVehicle.VehicleMovement` (`self.VehicleReference`)))))

(event `Key|P`
  (params (Key :type "Key Structure" :default "AnyKey"))
  (:`Pressed`
    (`KismetSystemLibrary.PrintString` (`KismetStringLibrary.Conv_DoubleToString` (`self.Lap3Time`)))
    (`KismetSystemLibrary.PrintString` (`KismetStringLibrary.Conv_DoubleToString` (`self.Lap2Time`)))
    (`KismetSystemLibrary.PrintString` (`KismetStringLibrary.Conv_DoubleToString` (`self.Lap1Time`)))))

(event `StartGameSetup`
  ;[1 1 1] Check for save and Init Text
  (`self.SaveGameCheck`)
  (`self.InitText`))

(event `Restart`
  ;[1 1 1] Restart map when race is finished after delay
  (`KismetSystemLibrary.Delay` (`self.CameraDelay`))
  (set `self.RaceStart` false)
  (`KismetSystemLibrary.ExecuteConsoleCommand` "RestartLevel"))

(event `self.ReceiveBeginPlay`
  ;[1 1 1] Begin Play
  (bind _returnvalue (`|CreateWidget` "/Game/Blueprints/UI/HUD.HUD_C"))
  (bind _output_get (set `self.HUDReference` _returnvalue))
  (`UserWidget.AddToViewport` _output_get 0)
  (bind _asbp_buggey (cast `/Game/Buggey/BP_Buggey` (`GameplayStatics.GetPlayerPawn` 0)))
  (set `self.VehicleReference` _asbp_buggey))

(event `StartRaceTime`
  ;[1 1 1] Race and lap timers
  (bind (_direction _time) (`Timeline|GameTime` :!label _label)
    (:`Update`
      (bind _output_get (set `self.ActualRaceTime` _time))
      (set `self.RaceTimeText` (`/Game/Blueprints/TimeConversion.TimeToText` _output_get)))))

(event `UpdateLap`
  ;[1 1 1] Update lap and checks for new lap record
  (bind _output_get (set `self.ActualLap` (+ (`self.ActualLap`) 1)))
  (set `self.CurrentLapText` (`KismetTextLibrary.Conv_IntToText` _output_get))
  (`self.LapTimeCheck`))

(event `StopRaceTime`
  ;[1 1 1] Race and lap timers
  (goto _label :!via `Stop`))

(event `StartLapTime`
  ;[1 1 1] Race and lap timers
  (bind (_direction _time) (`Timeline|LapTime` :!via `PlayFromStart` :!label _label_2)
    (:`Update`
      (bind _output_get (set `self.ActualLapTime` _time))
      (set `self.CurrentLapTimeText` (`/Game/Blueprints/TimeConversion.TimeToText` _output_get)))))

(event `RespawnVehicle`
  ;[1 1 1] Respawn vehicle when flipped
  (bind _returnvalue (`|SpawnActorFromClass` "/Game/Buggey/BP_Buggey.BP_Buggey_C" (`KismetMathLibrary.MakeTransform` (.location (`self.ReSpawnLocation`)) (.rotation (`self.ReSpawnLocation`))) "Undefined" "OverrideRootScale"))
  (`self.Possess` _returnvalue))

(event `StopLapTime`
  ;[1 1 1] Race and lap timers
  (goto _label_2 :!via `Stop`))

(event `Key|R`
  (params (Key :type "Key Structure" :default "AnyKey"))
  ;[1 1 1] Reset the default times
  (:`Released`
    (if (not (`self.RaceStart`))
      (set `self.BestLapTime` (`self.DefaultBestLapTime`))
      (set `self.BestRaceTime` (`self.DefaultBestRaceTime`))
      (`self.SaveTheGame`)
      (`self.InitText`))))

(event `InputAction|RaceStart`
  (params (Key :type "Key Structure" :default "AnyKey"))
  (bind _hudreference (`self.HUDReference`))
  (:`Pressed`
    ;[1 1 1] left click to start or restart the race
    (if (`self.RaceComplete`)
      (set `self.ShowWorldCamera` true)
      (`self.Restart`)
      (else
        (set `self.ShowWorldCamera` false)
        (`/Engine/EditorBlueprintResources/StandardMacros.DoOnce` false
          (:`Completed`
            (set `/Game/Blueprints/UI/HUD.SplashScreenVisible` "Hidden" _hudreference)
            (`KismetSystemLibrary.Delay` (`self.CameraDelay`))
            (set `/Game/Blueprints/UI/HUD.CountdownVisible` "Visible" _hudreference)
            (set `/Game/Blueprints/UI/HUD.GameHudVisible` "Visible" _hudreference)
            (`KismetSystemLibrary.Delay` 1.0)
            (set `self.Countdown` 2)
            (`KismetSystemLibrary.Delay` 1.0)
            (set `self.Countdown` 1)
            (`KismetSystemLibrary.Delay` 1.0)
            (set `self.Countdown` 0)
            (set `self.RaceStart` true)
            (`self.StartRaceTime`)
            (`self.StartLapTime`)
            (`KismetSystemLibrary.Delay` 2.0)
            (set `/Game/Blueprints/UI/HUD.CountdownVisible` "Hidden" (`self.HUDReference`))))))))

(fn `InitText`
  ;[1 1 1] Converts numerical values into text
  (set `self.CurrentLapText` (`KismetTextLibrary.Conv_IntToText` (`self.ActualLap`)))
  (set `self.MaxLapText` (`KismetTextLibrary.Conv_IntToText` (`self.MaxLaps`)))
  (set `self.GoldTimeText` (`/Game/Blueprints/TimeConversion.TimeToText` (`self.GoldTime`)))
  (set `self.SilverLapText` (`/Game/Blueprints/TimeConversion.TimeToText` (`self.SilverTime`)))
  (set `self.BronzeLapText` (`/Game/Blueprints/TimeConversion.TimeToText` (`self.BronzeTime`)))
  (set `self.BestLapText` (`/Game/Blueprints/TimeConversion.TimeToText` (`self.BestLapTime`)))
  (set `self.BestTimeText` (`/Game/Blueprints/TimeConversion.TimeToText` (`self.BestRaceTime`)))
  (set `self.CurrentLapTimeText` (`/Game/Blueprints/TimeConversion.TimeToText` (`self.ActualLapTime`)))
  (set `self.RaceTimeText` (`/Game/Blueprints/TimeConversion.TimeToText` (`self.ActualRaceTime`)))
  (set `self.Lap1TimeText` (`/Game/Blueprints/TimeConversion.TimeToText` (`self.Lap1Time`)))
  (set `self.Lap2TimeText` (`/Game/Blueprints/TimeConversion.TimeToText` (`self.Lap2Time`)))
  (set `self.Lap3TimeText` (`/Game/Blueprints/TimeConversion.TimeToText` (`self.Lap3Time`))))

(fn `LapTimeCheck`
  (bind _hudreference (`self.HUDReference`))
  (bind _hudreference_2 (`self.HUDReference`))
  (bind _hudreference_3 (`self.HUDReference`))
  (bind _actuallaptime (`self.ActualLapTime`))
  ;[1 1 1] Check if we have a new lap record and saves. Calls restart lap time
  (`self.StopLapTime`)
  (switch `int` (- (`self.ActualLap`) 1)
    (:`1`
      (set `self.Lap1Time` _actuallaptime))
    (:`2`
      (set `self.Lap2Time` _actuallaptime))
    (:`3`
      (set `self.Lap3Time` _actuallaptime)))
  (if (< (`self.ActualLapTime`) (`self.BestLapTime`))
    (bind _output_get (set `self.BestLapTime` (`self.ActualLapTime`)))
    (set `self.BestLapText` (`/Game/Blueprints/TimeConversion.TimeToText` _output_get))
    (`self.SaveTheGame`)
    (`UserWidget.PlayAnimation` _hudreference_2 (`/Game/Blueprints/UI/HUD.LapAnimation` _hudreference_2) 0.0 1 "Forward")
    (set `/Game/Blueprints/UI/HUD.NewLapRecordVisible` "Visible" (`self.HUDReference`))
    (set `self.ActualLapTime` 0.0)
    (else
      (set `self.ActualLapTime` 0.0)))
  (if (`self.RaceComplete`)
    (`self.RaceTimeCheck`)
    (else
      (`self.StartLapTime`)
      ;[1 1 1] Display lap number at the end of a lap
      (if (== (`self.ActualLap`) (`self.MaxLaps`))
        (`UserWidget.PlayAnimation` _hudreference (`/Game/Blueprints/UI/HUD.FinalLapAnimation` _hudreference) 0.0 1 "Forward")
        (else
          (`UserWidget.PlayAnimation` _hudreference_3 (`/Game/Blueprints/UI/HUD.NextLapAnimation` _hudreference_3) 0.0 1 "Forward"))))))

(fn `LoadTheGame`
  ;[1 1 1] Loads the game from MySaveGame
  (bind _returnvalue (`GameplayStatics.LoadGameFromSlot` (`self.SaveSlot`)))
  (bind _asmy_save_game (cast `/Game/Blueprints/MySaveGame` _returnvalue))
  (set `self.BestRaceTime` (`/Game/Blueprints/MySaveGame.SavedBestTime` _asmy_save_game))
  (set `self.BestLapTime` (`/Game/Blueprints/MySaveGame.SavedBestLap` _asmy_save_game)))

(fn `RaceTimeCheck`
  (bind _hudreference (`self.HUDReference`))
  ;[1 1 1] Checks if we have a new best time and saves if true
  (`self.StopRaceTime`)
  (if (< (`self.ActualRaceTime`) (`self.BestRaceTime`))
    (bind _output_get (set `self.BestRaceTime` (`self.ActualRaceTime`)))
    (set `self.BestTimeText` (`/Game/Blueprints/TimeConversion.TimeToText` _output_get))
    (set `/Game/Blueprints/UI/HUD.NewRaceRecordVisible` "Visible" (`self.HUDReference`))
    (`self.SaveTheGame`))
  (`self.InitText`)
  (set `/Game/Blueprints/UI/HUD.GameHudVisible` "Hidden" _hudreference)
  (set `/Game/Blueprints/UI/HUD.ResultsScreenVisible` "Visible" _hudreference))

(fn `SaveGameCheck`
  ;[1 1 1] Check if a save exists
  (bind _returnvalue (`GameplayStatics.DoesSaveGameExist` (`self.SaveSlot`)))
  (if _returnvalue
    (`self.LoadTheGame`)
    (else
      (set `self.BestLapTime` (`self.DefaultBestLapTime`))
      (set `self.BestRaceTime` (`self.DefaultBestRaceTime`))
      (`self.SaveTheGame`))))

(fn `SaveTheGame`
  ;[1 1 1] Saves the Game
  (bind _returnvalue (`GameplayStatics.CreateSaveGameObject` "/Game/Blueprints/MySaveGame.MySaveGame_C"))
  (bind _output_get (set `self.SaveGameReference` _returnvalue))
  (bind _asmy_save_game (cast `/Game/Blueprints/MySaveGame` _output_get))
  (set `/Game/Blueprints/MySaveGame.SavedBestLap` (`self.BestLapTime`) _asmy_save_game)
  (set `/Game/Blueprints/MySaveGame.SavedBestTime` (`self.BestRaceTime`) _asmy_save_game)
  (`GameplayStatics.SaveGameToSlot` (`self.SaveGameReference`) (`self.SaveSlot`)))

(fn `UserConstructionScript`)