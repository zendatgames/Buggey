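; Tennis ball racetrack obstacle that slows the player's buggy when a vehicle touches it.
; Every tick it tests its collision sphere's shape at the FurBall component's location for Vehicle objects.
; On a hit it quarters the linear velocity of player 0's BP_Buggey, whichever vehicle overlapped.
; A CanCollide flag blocks repeat hits until a four-second timer calls ResetCanCollide.
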(event `self.ReceiveTick`
  (params (DeltaSeconds :type "Float (single-precision)"))
  (bind (_outactors _returnvalue) (`KismetSystemLibrary.ComponentOverlapActors_NEW` (`self.CollisionSphere`) (`KismetMathLibrary.Conv_VectorToTransform` (`SceneComponent.K2_GetComponentLocation` (`self.FurBall`))) (`|MakeArray` "ObjectTypeQuery5" :!type "EObjectTypeQuery Enum")))
  (if (and _returnvalue (`self.CanCollide`))
    (set `self.CanCollide` false)
    (bind _asbp_buggey (cast `/Game/Buggey/BP_Buggey` (`GameplayStatics.GetPlayerPawn` 0)))
    (bind _mesh (`WheeledVehicle.Mesh` _asbp_buggey))
    (bind _returnvalue_2 (`PrimitiveComponent.GetPhysicsLinearVelocity` _mesh "None"))
    (`PrimitiveComponent.SetPhysicsLinearVelocity` _mesh (* _returnvalue_2 0.25) false "None")
    (`KismetSystemLibrary.K2_SetTimer` null "ResetCanCollide" 4.0)))

(fn `ResetCanCollide`
  (set `self.CanCollide` true))

(fn `UserConstructionScript`)