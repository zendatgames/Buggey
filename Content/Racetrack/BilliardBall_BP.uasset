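; BilliardBall_BP is a billiard ball actor that picks its appearance from a tag and can drop into a pocket.
; On BeginPlay it converts its first tag to an integer and uses it as an index into MeshArray to set the static mesh.
; The UnlockZ event clears the mesh's constraint mode, freeing the Z axis so the ball can fall.
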(event `UnlockZ`
  ;[1 1 1] Unlock the Z axis to fall in Pocket
  (`PrimitiveComponent.SetConstraintMode` (`self.StaticMesh`) "None"))

(event `self.ReceiveBeginPlay`
  ;[1 1 1] Set the mesh based on Tag at game start
  (`StaticMeshComponent.SetStaticMesh` (`self.StaticMesh`) (`KismetArrayLibrary.Array_Get` (`self.MeshArray`) (`KismetStringLibrary.Conv_StringToInt` (`KismetStringLibrary.Conv_NameToString` (`KismetArrayLibrary.Array_Get` (`self.Tags`)))))))

(fn `UserConstructionScript`)